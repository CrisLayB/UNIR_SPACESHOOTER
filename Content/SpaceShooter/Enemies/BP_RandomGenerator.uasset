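; BP_RandomGenerator is the Space Shooter enemy spawner, creating ships on a looping timer while EnemiesDestroyed is below MaxNumEnemies.
; Each spawn picks a random scene component tagged SpawnPoint and a class index randomized by the game mode's Level.
; Both class options currently resolve to BP_Enemy_Ship_Normal.
; Each enemy's OnDestroyed binds to an empty handler; the kill-count and level logic is disconnected, so the spawn limit never advances.
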(event Custom|Spawn
  (if (< (Variables|Default|GetEnemiesDestroyed) (Variables|Default|GetMaxNumEnemies))
    (bind _enemy_spawned (CallFunction|SpawnEnemy))
    (bind _asbp_enemy_base (Utilities|Casting|CastToBP_Enemy_Base _enemy_spawned))
    (Game|BindEventtoOnDestroyed _asbp_enemy_base (delegate Custom|EnemyDestroyed))))

(event Custom|EnemyDestroyed
  (params (DestroyedActor :type Actor%20Object%20Reference)))

(event EventBeginPlay
  (Utilities|Time|SetTimerbyEvent (delegate Custom|Spawn) (Variables|Default|GetSpawnTime) true)
  (bind _asss_game_mode (Utilities|Casting|CastToSS_GameMode (Game|GetGameMode)))
  (Variables|Default|SetSS%20Game%20Mode _asss_game_mode))

(fn ConstructionScript)

(fn SpawnEnemy
  (bind _returnvalue (Actor|GetComponentsbyTag "/Script/Engine.SceneComponent" "SpawnPoint"))
  (bind _class (CallFunction|GetClasstoSpawn (Math|Random|RandomInteger (Variables|/Game/SpaceShooter/SS_GameMode.SS_GameMode_C|GetLevel (Variables|Default|GetSS%20Game%20Mode)))))
  (bind _asscene_component (Utilities|Casting|CastToSceneComponent (Utilities|Array|Get(acopy) _returnvalue (Math|Random|RandomInteger (Utilities|Array|Length _returnvalue)))))
  (bind _returnvalue_2 (Game|SpawnActorfromClass _class (Transformation|GetWorldTransform _asscene_component) "Undefined" "MultiplyWithRoot" 0 0))
  (bind _asbp_enemy_base (Utilities|Casting|CastToBP_Enemy_Base _returnvalue_2))
  (return _asbp_enemy_base))

(fn GetClasstoSpawn
  (params (Type :type Integer))
  (return (Utilities|Select :Index (Math|Integer|Clamp(Integer) Type 0 (- (Variables|Default|GetMaxNumEnemies) 0)) :Option%200 "/Game/SpaceShooter/Enemies/BP_Enemy_Ship_Normal.BP_Enemy_Ship_Normal_C" :Option%201 "/Game/SpaceShooter/Enemies/BP_Enemy_Ship_Normal.BP_Enemy_Ship_Normal_C")))